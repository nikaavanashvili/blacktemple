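; BP_minecharacter is a player character Blueprint that handles movement and sprinting through Enhanced Input.
; BeginPlay adds the default mapping context to the first player controller's input subsystem.
; The move action feeds its swapped X/Y axes into world-space movement, independent of camera facing, while the sprint action switches max walk speed between fast and normal.
; An unconnected fragment for setting control rotation never runs.
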(event Input|EnhancedActionEvents|EnhancedInputActionAI_sriftspeed
  (params (ActionValue :type Boolean) (ElapsedSeconds :type Float%20%28double-precision%29) (TriggeredSeconds :type Float%20%28double-precision%29) (InputAction :type Input%20Action%20Object%20Reference :default "/Game/input/AI_sriftspeed.AI_sriftspeed"))
  ;[0.15 0.15 0.15 0.5] max walk speed
  (:Triggered
    (Variables|/Script/Engine.CharacterMovementComponent|SetMaxWalkSpeed (Variables|Character|GetCharacterMovement) (Math|Float|SelectFloat 666.0 333.0 ActionValue) :!label _label))
  (:Started
    (goto _label))
  (:Ongoing
    (goto _label))
  (:Canceled
    (goto _label))
  (:Completed
    (goto _label)))

(event Input|EnhancedActionEvents|EnhancedInputActionAI_muve
  (params (ActionValue :type Vector%202D%20Structure) (ElapsedSeconds :type Float%20%28double-precision%29) (TriggeredSeconds :type Float%20%28double-precision%29) (InputAction :type Input%20Action%20Object%20Reference :default "/Game/input/AI_muve.AI_muve"))
  (bind (_x _y) (Math|Vector2D|BreakVector2D ActionValue))
  ;[0.15 0.15 0.15 0.5] add muve input
  (Pawn|Input|AddMovementInput (Math|Vector|MakeVector _y _x 0.0) 1.0 false))

(event EventBeginPlay
  ;[0.15 0 0.07215 0.5] ADDING MAPPING CONTEXT ON BEGYNPLAY
  (Input|AddMappingContext (PlayerController|LocalPlayerSubsystems|GetEnhancedInputLocalPlayerSubsystem (Game|GetPlayerController 0)) "/Game/input/IMS_default.IMS_default" 0 "(bIgnoreAllPressedKeysUntilRelease=True,bForceImmediately=False,bNotifyUserSettings=False)"))

(fn ConstructionScript)