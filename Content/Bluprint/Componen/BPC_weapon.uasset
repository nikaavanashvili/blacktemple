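; Weapon component that gives its owner a visible gun (commented as an AK47) and handles firing.
; BeginPlay spawns a skeletal mesh actor, async-loads the weapon mesh, attaches it to the owner's weapon_socket without collision, and adds the IMS_Weapon input context for player 0.
; The fire input spawns BP_WeaponBullet at the Muzzle socket, using only the weapon's yaw for direction.
; EndPlay removes the input context.
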(event Input|EnhancedActionEvents|EnhancedInputActionAI_WeaponFire
  (params (ActionValue :type Boolean) (ElapsedSeconds :type Float%20%28double-precision%29) (TriggeredSeconds :type Float%20%28double-precision%29) (InputAction :type Input%20Action%20Object%20Reference :default "/Game/input/inputactions/AI_WeaponFire.AI_WeaponFire"))
  (bind _skeletal_mesh_component (Variables|Default|GetSkeletal%20Mesh%20Component))
  (Game|SpawnActorfromClass "/Game/Bluprint/Weapon/BP_WeaponBullet.BP_WeaponBullet_C" (Math|Transform|MakeTransform (Transformation|GetSocketLocation (.ReturnValue (Class|SkeletalMesh|FindSocketandIndex (Variables|Default|GetAs%20Skeletal%20Mesh) "Muzzle")) _skeletal_mesh_component) (Math|Rotator|MakeRotator 0.0 0.0 (.yaw (Transformation|GetWorldRotation _skeletal_mesh_component)))) "AlwaysSpawn" "MultiplyWithRoot" 0 0))

(event EventBeginPlay
  (bind _returnvalue (Components|GetOwner))
  ;[0.15 0 0.1313 0.5] Event Begin Play Weapon Ak47
  (Utilities|FlowControl|Sequence
    (:then_0
      (bind _returnvalue_2 (Game|SpawnActorfromClass "/Script/Engine.SkeletalMeshActor" (Math|Transform|MakeTransform "0, 0, 0") "AlwaysSpawn" "MultiplyWithRoot" _returnvalue (.AsPawn (Utilities|Casting|CastToPawn _returnvalue))))
      (Variables|Default|SetSkeletal%20Mesh%20Component (Variables|/Script/Engine.SkeletalMeshActor|GetSkeletalMeshComponent _returnvalue_2))
      (bind _object (Utilities|AsyncLoadAsset (Variables|Default|Getweapon))
        (:Completed
          (Variables|Default|SetAs%20Skeletal%20Mesh (.AsSkeletal%20Mesh (Utilities|Casting|CastToSkeletalMesh _object)))
          (Components|SkeletalMesh|SetSkeletalMeshAsset (Variables|Default|GetSkeletal%20Mesh%20Component) (.AsSkeletal%20Mesh (Utilities|Casting|CastToSkeletalMesh _object)))
          (Transformation|AttachComponentToComponent _returnvalue_2 (Actor|GetComponentbyClass (Components|GetOwner) "/Script/Engine.SkeletalMeshComponent") "weapon_socket" "SnapToTarget" "SnapToTarget" "SnapToTarget" true)
          (Collision|SetCollisionEnabled (Variables|Default|GetSkeletal%20Mesh%20Component) "NoCollision"))))
    (:then_1
      (Input|AddMappingContext (PlayerController|LocalPlayerSubsystems|GetEnhancedInputLocalPlayerSubsystem (Game|GetPlayerController 0)) "/Game/input/IMS_Weapon.IMS_Weapon" 1 "(bIgnoreAllPressedKeysUntilRelease=True,bForceImmediately=False,bNotifyUserSettings=False)"))))

(event EventEndPlay
  (params (EndPlayReason :type EEndPlayReason%20Enum :default "Destroyed"))
  (bind _returnvalue (Game|GetPlayerController 0))
  (bind _returnvalue_2 (PlayerController|LocalPlayerSubsystems|GetEnhancedInputLocalPlayerSubsystem _returnvalue))
  ;[0.15 0 0.07215 0.5] End Play Remove Mapping Context
  (Utilities|IsValid _returnvalue_2
    (:Is%20Valid
      (Input|RemoveMappingContext _returnvalue_2 "/Game/input/IMS_Weapon.IMS_Weapon" "(bIgnoreAllPressedKeysUntilRelease=True,bForceImmediately=False,bNotifyUserSettings=False)"))))