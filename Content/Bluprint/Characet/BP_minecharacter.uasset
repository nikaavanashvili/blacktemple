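; Player character Blueprint with mouse-cursor-directed movement, sprinting and jumping through Enhanced Input.
; BeginPlay adds the base mapping context and shows the cursor.
; The move action pushes the character along its capsule's forward vector, turns control rotation toward the cursor's trace hit, flattened to actor height, and draws a debug sphere there.
; The sprint action switches max walk speed between two values, and the jump action starts or stops jumping.
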(event Input|EnhancedActionEvents|EnhancedInputActionAI_sriftspeed
  (params (ActionValue :type Boolean) (ElapsedSeconds :type Float%20%28double-precision%29) (TriggeredSeconds :type Float%20%28double-precision%29) (InputAction :type Input%20Action%20Object%20Reference :default "/Game/input/inputactions/AI_sriftspeed.AI_sriftspeed"))
  ;[0.15 0.15 0.15 0.5] max walk speed
  (:Triggered
    (Variables|/Script/Engine.CharacterMovementComponent|SetMaxWalkSpeed (Variables|Character|GetCharacterMovement) (Math|Float|SelectFloat 6e+02 3e+02 ActionValue) :!label _label))
  (:Started
    (goto _label))
  (:Ongoing
    (goto _label))
  (:Canceled
    (goto _label))
  (:Completed
    (goto _label)))

(event Input|EnhancedActionEvents|EnhancedInputActionAI_Jomp
  (params (ActionValue :type Boolean) (ElapsedSeconds :type Float%20%28double-precision%29) (TriggeredSeconds :type Float%20%28double-precision%29) (InputAction :type Input%20Action%20Object%20Reference :default "/Game/input/inputactions/AI_Jomp.AI_Jomp"))
  (:Triggered
    (Character|Jump))
  (:Canceled
    (Character|StopJumping)))

(event Input|EnhancedActionEvents|EnhancedInputActionAI_muve
  (params (ActionValue :type Float%20%28double-precision%29) (ElapsedSeconds :type Float%20%28double-precision%29) (TriggeredSeconds :type Float%20%28double-precision%29) (InputAction :type Input%20Action%20Object%20Reference :default "/Game/input/inputactions/AI_muve.AI_muve"))
  (bind _returnvalue (Transformation|GetActorLocation))
  (bind _returnvalue_2 (Game|GetPlayerController 0))
  (bind _hitresult (Game|Player|GetHitResultUnderCursorbyChannel _returnvalue_2 "TraceTypeQuery1" true))
  (bind _z (Math|Vector|BreakVector _returnvalue))
  (bind _impactpoint (Collision|BreakHitResult _hitresult))
  (bind _returnvalue_3 (Math|Vector|MakeVector (.x _impactpoint) (.y _impactpoint) _z))
  ;[0.15 0.15 0.15 0.5] add muve input
  (Pawn|Input|AddMovementInput (Math|Vector|GetForwardVector (Variables|Collision|GetCapsuleComponent)) ActionValue false)
  (Pawn|SetControlRotation (Pawn|GetController) (Math|Rotator|FindLookatRotation _returnvalue _returnvalue_3))
  (Rendering|Debug|DrawDebugSphere _returnvalue_3 1e+02 12 "(R=1.000000,G=1.000000,B=1.000000,A=1.000000)" 0.0))

(event EventBeginPlay
  ;[0.15 0 0.07215 0.5] ADDING MAPPING CONTEXT ON BEGYNPLAY
  (Input|AddMappingContext (PlayerController|LocalPlayerSubsystems|GetEnhancedInputLocalPlayerSubsystem (Game|GetPlayerController 0)) "/Game/input/IMS_Basemapping.IMS_Basemapping" 0 "(bIgnoreAllPressedKeysUntilRelease=True,bForceImmediately=False,bNotifyUserSettings=False)")
  (Variables|/Script/Engine.PlayerController|SetbShowMouseCursor (Game|GetPlayerController 0) true))

(fn ConstructionScript)